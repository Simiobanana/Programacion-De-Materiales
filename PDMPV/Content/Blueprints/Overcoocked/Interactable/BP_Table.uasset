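; BP_Table is an interactable table in the Overcoocked game that holds one object for players to drop off or pick up.
; On GrabDrop, a player carrying an object places it if the table is empty, attaching it to the target component, sliding it with MoveComponentTo and clearing the player's hold.
; An empty-handed player instead grabs the placed object, which frees the table.
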(event EventBeginPlay)

(event EventGrabDrop
  (params (Player :type BP%20Character%20Object%20Reference))
  (bind (_returnvalue _grabbedobject) (Default|GetGrabbedObject Player))
  (if _returnvalue
    (Utilities|IsValid (Variables|Default|GetPlacedTarget)
      (:Is%20Not%20Valid
        (bind _output_get (Variables|Default|SetPlacedTarget _grabbedobject))
        (Transformation|AttachComponentToComponent _output_get (Variables|Default|GetTarget) "None" "KeepWorld" "KeepWorld" "KeepWorld" true)
        (Components|MoveComponentTo (Variables|/Script/Engine.Actor|GetRootComponent (Variables|Default|GetPlacedTarget)) "0, 0, 0" "0, 0, 0" false false 0.2 false)
        (Variables|/Game/Blueprints/Overcoocked/BP_Character.BP_Character_C|SetGrabbedObject Player 0)))
    (else
      ;[1 0.8584 0] Grab Objects From The Table
      (Utilities|IsValid (Variables|Default|GetPlacedTarget)
        (:Is%20Valid
          (Default|Grab Player (Variables|Default|GetPlacedTarget))
          (Variables|Default|SetPlacedTarget 0))))))

(fn ConstructionScript)