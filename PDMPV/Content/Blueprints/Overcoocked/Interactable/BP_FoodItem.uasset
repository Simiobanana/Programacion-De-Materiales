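; BP_FoodItem is an interactable food item for the Overcoocked game that tracks a Raw, Slicing or Sliced preparation state.
; SetState stores the new state and swaps the Sphere mesh's material to match it.
; CanBeSliced returns only the IsSlicable flag; a state-based check that would exclude Sliced items is present but unconnected.
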(event Custom|SetState
  (params (State :type BPE_FoodItemStates%20Enum :default "NewEnumerator0"))
  (bind _output_get (Variables|Default|SetState State))
  (Rendering|Material|SetMaterial (Variables|Default|GetSphere) 0 (Utilities|Select :Index _output_get :NewEnumerator0 "/Game/Materials/BaseColor/Raw.Raw" :NewEnumerator1 "/Game/Materials/BaseColor/Cafe.Cafe" :NewEnumerator2 "/Game/Materials/BaseColor/Sliced.Sliced")))

(event EventBeginPlay)

(event Collision|EventActorBeginOverlap
  (params (OtherActor :type Actor%20Object%20Reference)))

(event EventTick
  (params (DeltaSeconds :type Float%20%28single-precision%29)))

(fn ConstructionScript
  (|CallParentFunction))

(fn CanbeSliced
  (return (Variables|Default|GetIsSlicable)))