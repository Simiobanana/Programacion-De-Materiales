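; BP_Grabbable is an interactable object that a player can pick up and drop.
; GrabDrop acts only when the player holds nothing: it turns off physics and collision on the root, then calls the player's Grab with itself.
; Drop detaches the object at its world transform and re-enables physics simulation, but sets collision to NoCollision again rather than restoring it.
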(event Custom|Drop
  (bind _root (Variables|Default|GetRoot))
  ;[0.2286 0 1] Detach From Actor
  (Transformation|DetachFromActor "KeepWorld" "KeepWorld" "KeepWorld")
  (Physics|SetSimulatePhysics _root true)
  (Collision|SetCollisionEnabled _root "NoCollision"))

(event EventGrabDrop
  (params (Player :type BP%20Character%20Object%20Reference))
  (bind _root (Variables|Default|GetRoot))
  ;[1 0.8252 0] Set Object Interaction
  (if (not (.ReturnValue (Default|GetGrabbedObject Player)))
    (Physics|SetSimulatePhysics _root false)
    (Collision|SetCollisionEnabled _root "NoCollision")
    (Default|Grab Player self)))

(fn ConstructionScript)