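; Player character for an Overcooked-style game that moves, interacts with objects and carries one in its hands.
; Enhanced Input drives movement and triggers a short sphere trace ahead of the character, ignoring the held object.
; A hit receives an Interact message with the character as argument; a miss drops any held object.
; Grab stores the given object, attaches it to the Hands component and calls MoveComponentTo on its root.
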(event Custom|Grab
  (params (Object%20To%20Grab :type BP%20Grabbable%20Object%20Reference))
  ;[1 0 0.26] Grab Objects To Actor
  (bind _output_get (Variables|Default|SetGrabbedObject Object%20To%20Grab))
  (Transformation|AttachComponentToComponent _output_get (Variables|Default|GetHands) "None" "KeepWorld" "KeepWorld" "KeepWorld" true)
  (Components|MoveComponentTo (Variables|/Script/Engine.Actor|GetRootComponent (Variables|Default|GetGrabbedObject)) "0, 0, 0" "0, 0, 0" false false 0.2 false))

(event Input|EnhancedActionEvents|EnhancedInputActionIA_MovementOvercoocked
  (params (ActionValue :type Vector%202D%20Structure) (ElapsedSeconds :type Float%20%28double-precision%29) (TriggeredSeconds :type Float%20%28double-precision%29) (InputAction :type Input%20Action%20Object%20Reference :default "/Game/Inputs/IA_MovementOvercoocked.IA_MovementOvercoocked"))
  ;[1 0.4117 0.003422] Character_Input_Movement
  (Pawn|Input|AddMovementInput (Math|Conversions|ToVector(Vector2D) ActionValue) 1.0 false))

(event Input|EnhancedActionEvents|EnhancedInputActionIA_Interaction
  (params (ActionValue :type Boolean) (ElapsedSeconds :type Float%20%28double-precision%29) (TriggeredSeconds :type Float%20%28double-precision%29) (InputAction :type Input%20Action%20Object%20Reference :default "/Game/Inputs/IA_Interaction.IA_Interaction"))
  (bind (_returnvalue _grabbedobject) (CallFunction|GetGrabbedObject))
  (bind _returnvalue_2 (Transformation|GetActorForwardVector))
  (bind _returnvalue_3 (Transformation|GetActorLocation))
  (bind _returnvalue_4 (* _returnvalue_2 5e+01))
  (bind _returnvalue_5 (+ _returnvalue_4 _returnvalue_3))
  (bind (_x _y _z) (Math|Vector|BreakVector _returnvalue_5))
  ;[0.01423 0 1] Character Interaction
  (:Started
    (bind (_outhit _returnvalue_6) (Collision|SphereTraceByChannel (Math|Vector|MakeVector _x _y (+ _z -5e+01)) (Math|Vector|MakeVector _x _y (+ _z 1e+01)) 3e+01 "TraceTypeQuery3" false (Utilities|Array|MakeArray (Variables|Default|GetGrabbedObject)) "ForDuration"))
    (if _returnvalue_6
      (Class|BPIInteractable|Interact(Message) (.HitActor (Collision|BreakHitResult _outhit)) self)
      (elif _returnvalue
        (Default|Drop _grabbedobject)
        (Variables|Default|SetGrabbedObject 0)))))

(fn ConstructionScript)

(fn GetGrabbedObject
  (bind _grabbedobject (Variables|Default|GetGrabbedObject))
  (return (Utilities|IsValid _grabbedobject) _grabbedobject))