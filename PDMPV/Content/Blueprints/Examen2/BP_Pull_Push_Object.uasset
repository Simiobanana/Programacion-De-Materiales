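; Pushable and pullable box that the third-person character moves by interacting with it.
; Overlapping the Forward component sets the character's CanInteractingBox flag, without checking which actor overlaps.
; While that and IsInteractingBox are true, Tick reads both input axes and calls SpeedDirection with fixed signed speeds.
; SpeedDirection eases Base's relative location with VInterpTo and no sweep, using its right vector for forward/backward and forward vector for left/right.
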(event OnComponentBeginOverlap(Forward)
  (params (OverlappedComponent :type Primitive%20Component%20Object%20Reference) (OtherActor :type Actor%20Object%20Reference) (OtherComp :type Primitive%20Component%20Object%20Reference) (OtherBodyIndex :type Integer) (bFromSweep :type Boolean) (SweepResult :type Hit%20Result%20Structure%20%28by%20ref%29))
  (Development|PrintString "Hello" true true "(R=0.000000,G=0.660000,B=1.000000,A=1.000000)" 2.0 "2345654")
  (Variables|/Game/ThirdPerson/Blueprints/BP_ThirdPersonCharacter.BP_ThirdPersonCharacter_C|SetCanInteractingBox? (Variables|Default|GetCharacterREF) true))

(event OnComponentEndOverlap(Forward)
  (params (OverlappedComponent :type Primitive%20Component%20Object%20Reference) (OtherActor :type Actor%20Object%20Reference) (OtherComp :type Primitive%20Component%20Object%20Reference) (OtherBodyIndex :type Integer))
  (Development|PrintString "Character can interact" true true "(R=0.000000,G=0.660000,B=1.000000,A=1.000000)" 2.0 "3234564564")
  (Variables|/Game/ThirdPerson/Blueprints/BP_ThirdPersonCharacter.BP_ThirdPersonCharacter_C|SetCanInteractingBox? (Variables|Default|GetCharacterREF) false))

(event EventBeginPlay
  (bind _returnvalue (Actor|GetActorOfClass "/Game/ThirdPerson/Blueprints/BP_ThirdPersonCharacter.BP_ThirdPersonCharacter_C"))
  (Variables|Default|SetCharacterREF _returnvalue))

(event Collision|EventActorBeginOverlap
  (params (OtherActor :type Actor%20Object%20Reference)))

(event EventTick
  (params (DeltaSeconds :type Float%20%28single-precision%29))
  (bind _characterref (Variables|Default|GetCharacterREF))
  (bind _characterref_2 (Variables|Default|GetCharacterREF))
  (bind _action_value_x (Variables|/Game/ThirdPerson/Blueprints/BP_ThirdPersonCharacter.BP_ThirdPersonCharacter_C|GetAction%20Value%20X _characterref_2))
  (bind _action_value_y (Variables|/Game/ThirdPerson/Blueprints/BP_ThirdPersonCharacter.BP_ThirdPersonCharacter_C|GetAction%20Value%20Y _characterref_2))
  (if (Variables|/Game/ThirdPerson/Blueprints/BP_ThirdPersonCharacter.BP_ThirdPersonCharacter_C|GetIsInteractingBox? _characterref)
    (if (Variables|/Game/ThirdPerson/Blueprints/BP_ThirdPersonCharacter.BP_ThirdPersonCharacter_C|GetCanInteractingBox? _characterref)
      (Utilities|FlowControl|Sequence
        (:then_0
          (if (== _action_value_y 0.0)
            (Development|PrintString "is not moving")
            (elif (>= _action_value_y 0.1)
              (Development|PrintString "forward")
              (Utilities|SpeedDirection true 34.0)
              (else
                (Development|PrintString "Backward")
                (Utilities|SpeedDirection true -34.0)))))
        (:then_1
          (if (== _action_value_x 0.0)
            (Development|PrintString "is not moving")
            (elif (>= _action_value_x 0.1)
              (Development|PrintString "right")
              (Utilities|SpeedDirection false 5e+01)
              (else
                (Development|PrintString "left")
                (Utilities|SpeedDirection false -5e+01)))))))))

(fn ConstructionScript)